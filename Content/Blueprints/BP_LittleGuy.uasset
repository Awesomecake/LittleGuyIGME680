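; BP_LittleGuy is an actor with an XR root that places itself at a per-level camera starting position when play begins.
; After the parent BeginPlay, it looks up the current level name as a row in MapDataTable and moves to that row's CamStartingPosition.
; It then detaches XRRoot with world transform kept, decoupling it from later actor movement.
; Both steps run only when the row is found.
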(event EventBeginPlay
  (|CallParentFunction)
  (bind _returnvalue (Game|GetCurrentLevelName true))
  (bind _returnvalue_2 (Utilities|GetDataTableRow "/Game/Maps/MapData/MapDataTable.MapDataTable" (Utilities|String|StringToName _returnvalue))
    (:then
      (Transformation|SetActorLocation (.camstartingposition _returnvalue_2) false false)
      (Transformation|DetachFromComponent (Variables|Default|GetXRRoot) "KeepWorld" "KeepWorld" "KeepWorld" true))))

(event Collision|EventActorBeginOverlap
  (params (OtherActor :type Actor%20Object%20Reference))
  (|CallParentFunction OtherActor) ; This node is disabled and will not be called.\nDrag off pins to build functionality.
)

(event EventTick
  (params (DeltaSeconds :type Float%20%28single-precision%29))
  (|CallParentFunction DeltaSeconds) ; This node is disabled and will not be called.\nDrag off pins to build functionality.
)

(fn ConstructionScript
  (|CallParentFunction))
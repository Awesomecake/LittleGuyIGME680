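; BP_InteractionTrigger is a trigger zone that shows an interaction prompt to the third-person player.
; On box overlap, it pushes its InteractionText into the character's WB_InteractionPrompt widget and unhides the InteractPrompt component unless the character is grabbing.
; Leaving the box hides the prompt again.
; It only drives the prompt display and performs no interaction itself.
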(event OnComponentBeginOverlap(Box)
  (params (OverlappedComponent :type Primitive%20Component%20Object%20Reference) (OtherActor :type Actor%20Object%20Reference) (OtherComp :type Primitive%20Component%20Object%20Reference) (OtherBodyIndex :type Integer) (bFromSweep :type Boolean) (SweepResult :type Hit%20Result%20Structure%20%28by%20ref%29))
  ;[1 1 1] Toggle Interaction Prompt when Player is inside collision zone
  (bind _asbp_third_person_character (Utilities|Casting|CastToBP_ThirdPersonCharacter OtherActor))
  (bind _aswb_interaction_prompt (Utilities|Casting|CastToWB_InteractionPrompt (UserInterface|GetWidget (Variables|/Game/Blueprints/BP_ThirdPersonCharacter.BP_ThirdPersonCharacter_C|GetInteractPrompt _asbp_third_person_character))))
  (Default|ChangePromptText _aswb_interaction_prompt (Variables|Default|GetInteractionText))
  (if (not (Variables|/Game/Blueprints/BP_ThirdPersonCharacter.BP_ThirdPersonCharacter_C|GetisGrabbing _asbp_third_person_character))
    (Development|SetHiddeninGame (Variables|/Game/Blueprints/BP_ThirdPersonCharacter.BP_ThirdPersonCharacter_C|GetInteractPrompt _asbp_third_person_character) false false)))

(event OnComponentEndOverlap(Box)
  (params (OverlappedComponent :type Primitive%20Component%20Object%20Reference) (OtherActor :type Actor%20Object%20Reference) (OtherComp :type Primitive%20Component%20Object%20Reference) (OtherBodyIndex :type Integer))
  ;[1 1 1] Toggle Interaction Prompt when Player is inside collision zone
  (bind _asbp_third_person_character (Utilities|Casting|CastToBP_ThirdPersonCharacter OtherActor))
  (Development|SetHiddeninGame (Variables|/Game/Blueprints/BP_ThirdPersonCharacter.BP_ThirdPersonCharacter_C|GetInteractPrompt _asbp_third_person_character) true false))

(event EventBeginPlay)

(event Collision|EventActorBeginOverlap
  (params (OtherActor :type Actor%20Object%20Reference)))

(event EventTick
  (params (DeltaSeconds :type Float%20%28single-precision%29)))

(fn ConstructionScript)
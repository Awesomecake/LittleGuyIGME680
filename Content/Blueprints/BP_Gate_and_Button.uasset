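; BP_Gate_and_Button is a pressure button that moves a gate while any actor overlaps its box trigger.
; Begin and end overlaps maintain an actor list, so the gate reverses only when the last occupant leaves.
; GateMoveTimeline drives the gate mesh's Z scale, playing on entry and reversing on exit.
; The button mesh's Z scale switches between pressed and released, with X and Y set to zero both times.
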(event OnComponentBeginOverlap(Box)
  (params (OverlappedComponent :type Primitive%20Component%20Object%20Reference) (OtherActor :type Actor%20Object%20Reference) (OtherComp :type Primitive%20Component%20Object%20Reference) (OtherBodyIndex :type Integer) (bFromSweep :type Boolean) (SweepResult :type Hit%20Result%20Structure%20%28by%20ref%29))
  (bind _actors (Variables|Default|GetActors))
  (bind _sm_cube (Variables|Default|GetSM_Cube))
  (bind _relativescale3d (Variables|/Script/Engine.SceneComponent|GetRelativeScale3D _sm_cube))
  (Utilities|Array|Add _actors OtherActor)
  (bind _output_get (Variables|Default|SetExited false))
  (if (Math|Boolean|NORBoolean _output_get (Utilities|Array|IsEmpty _actors))
    (bind _output_get_2 (Variables|Default|SetButton%20Scale 0.0))
    (Transformation|SetRelativeScale3D (Variables|Default|GetSM_Cube2) (Math|Vector|MakeVector 0.0 0.0 _output_get_2))
    (bind _z_scale (Timeline|Gate%20Move%20Timeline Play)
      (:Update
        (Transformation|SetRelativeScale3D _sm_cube (Math|Vector|MakeVector (.x _relativescale3d) (.y _relativescale3d) _z_scale))))))

(event OnComponentEndOverlap(Box)
  (params (OverlappedComponent :type Primitive%20Component%20Object%20Reference) (OtherActor :type Actor%20Object%20Reference) (OtherComp :type Primitive%20Component%20Object%20Reference) (OtherBodyIndex :type Integer))
  (bind _actors (Variables|Default|GetActors))
  (bind _sm_cube (Variables|Default|GetSM_Cube))
  (bind _relativescale3d (Variables|/Script/Engine.SceneComponent|GetRelativeScale3D _sm_cube))
  (Utilities|Array|RemoveItem _actors OtherActor)
  (bind _output_get (Variables|Default|SetExited true))
  (if (and (Utilities|Array|IsEmpty _actors) _output_get)
    (bind _output_get_2 (Variables|Default|SetButton%20Scale 0.1))
    (Transformation|SetRelativeScale3D (Variables|Default|GetSM_Cube2) (Math|Vector|MakeVector 0.0 0.0 _output_get_2))
    (bind _z_scale (Timeline|Gate%20Move%20Timeline Reverse)
      (:Update
        (Transformation|SetRelativeScale3D _sm_cube (Math|Vector|MakeVector (.x _relativescale3d) (.y _relativescale3d) _z_scale))))))

(fn ConstructionScript)